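; Grappling hook projectile that pulls the player capsule to its location when it hits a BP_Target.
; Half a second after spawning, it eases back to the player unless HasCollided is set, then destroys itself.
; Hitting the player or ending overlap with them also destroys it, and destruction re-enables the character's CanShoot.
; Movement uses MoveComponentTo; some movement-mode and older grapple logic is left disconnected.
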(event Custom|MoveToPlayer
  ;[1 1 1] Return to player
  (if (not (Variables|Default|GetHasCollided))
    (bind _returnvalue (Actor|GetActorOfClass "/Game/ThirdPersonBP/Blueprints/ThirdPersonCharacter.ThirdPersonCharacter_C"))
    (Components|MoveComponentTo (Variables|MyProjectile|GetCollisionComponent) (Transformation|GetActorLocation _returnvalue) (Transformation|GetActorRotation) true true 0.5 false)
    (Variables|Default|SetHasCollided false)
    (Actor|DestroyActor) ; Then destroy this projectile
    (bind _returnvalue_2 (Actor|GetActorOfClass "/Game/ThirdPersonBP/Blueprints/ThirdPersonCharacter.ThirdPersonCharacter_C"))
    (Variables|/Game/ThirdPersonBP/Blueprints/ThirdPersonCharacter.ThirdPersonCharacter_C|SetCanShoot _returnvalue_2 true)))

(event Collision|EventActorEndOverlap
  (params (OtherActor :type Actor%20Object%20Reference))
  (bind _asthird_person_character (Utilities|Casting|CastToThirdPersonCharacter OtherActor))
  (Actor|DestroyActor)
  (Variables|/Game/ThirdPersonBP/Blueprints/ThirdPersonCharacter.ThirdPersonCharacter_C|SetCanShoot _asthird_person_character true))

(event EventBeginPlay
  ;[1 1 1] Trigger a return to the player after a duration
  (Utilities|FlowControl|Delay 0.5)
  (CallFunction|MovetoPlayer))

(event EventDestroyed
  (bind _returnvalue (Actor|GetActorOfClass "/Game/ThirdPersonBP/Blueprints/ThirdPersonCharacter.ThirdPersonCharacter_C"))
  (Variables|/Game/ThirdPersonBP/Blueprints/ThirdPersonCharacter.ThirdPersonCharacter_C|SetCanShoot _returnvalue true))

(event Collision|EventHit
  (params (MyComp :type Primitive%20Component%20Object%20Reference) (Other :type Actor%20Object%20Reference) (OtherComp :type Primitive%20Component%20Object%20Reference) (bSelfMoved :type Boolean) (HitLocation :type Vector :default "0, 0, 0") (HitNormal :type Vector :default "0, 0, 0") (NormalImpulse :type Vector :default "0, 0, 0") (Hit :type Hit%20Result%20Structure%20%28by%20ref%29))
  (bind _returnvalue (Game|GetPlayerCharacter 0))
  ;[1 1 1] Check if colliding
  (Utilities|Casting|CastToBP_Target Other
    (:then
      (Components|MoveComponentTo (Variables|/Script/Engine.Character|GetCapsuleComponent _returnvalue) (Transformation|GetActorLocation) (Transformation|GetActorRotation _returnvalue) true true 0.5 false))
    (:CastFailed
      (Utilities|Casting|CastToThirdPersonCharacter Other)
      (Actor|DestroyActor) ; Then destroy this projectile
    )))

(fn ConstructionScript)